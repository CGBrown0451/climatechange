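; Purifier device that accepts carried components from the player and offers a toggleable HUD.
; BeginPlay creates hidden HUD and display widgets; entering the overlap shows the display, leaving hides both.
; On overlap, the first BP_BaseObject overlapping the entering actor is matched by PurifierPart, destroyed and credited to BP_Char as hydraulic part, motor part or resources.
; InteractwithObject toggles the HUD, switching cursor and input mode accordingly.
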(event OnComponentBeginOverlap(Overlap)
  (params (OverlappedComponent :type Primitive%20Component%20Object%20Reference) (OtherActor :type Actor%20Object%20Reference) (OtherComp :type Primitive%20Component%20Object%20Reference) (OtherBodyIndex :type Integer) (bFromSweep :type Boolean) (SweepResult :type Hit%20Result%20Structure%20%28by%20ref%29))
  (bind _returnvalue (Game|GetPlayerCharacter 0))
  ;[1 1 1] Player-purifier interaction. Whenever the player is carrying an item. Delete the possessed item if it matches as purifier component. Otherwise ignore everything. Display the caption as soon player overlaps
  (Utilities|FlowControl|Sequence
    (:then_0
      ;;[1 1 1] Determine if anything is still interrupting
      (bind _output_get (Variables|Default|SetisHUDOpen true))
      (if _output_get
        (Widget|SetVisibility (Variables|Default|GetWBP_PurifierDisplay) "Hidden")))
    (:then_1
      (Widget|SetVisibility (Variables|Default|GetWBP_PurifierDisplay) "Visible")
      (bind _asbp_base_object (Utilities|Casting|CastToBP_BaseObject (Utilities|Array|Get(acopy) (Collision|GetOverlappingActors OtherActor "/Game/Blueprints/BP_BaseObject.BP_BaseObject_C" :!class /Script/Engine.Actor))))
      (bind _output_get_2 (Variables|Default|SetBP_BaseObjRef _asbp_base_object))
      (switch Utilities|FlowControl|Switch|SwitchonEnum_PuriferParts (.PurifierPart (Utilities|Struct|Breakstruct_PickupItem (Variables|/Game/Blueprints/BP_BaseObject.BP_BaseObject_C|GetItemInfo _output_get_2)))
        (:NewEnumerator0
          (Actor|DestroyActor (Variables|Default|GetBP_BaseObjRef))
          (Development|PrintString "A")
          (bind _asbp_char (Utilities|Casting|CastToBP_Char _returnvalue))
          (Default|AddHydraulicPart _asbp_char))
        (:NewEnumerator1
          (bind _asbp_char_2 (Utilities|Casting|CastToBP_Char (Game|GetPlayerCharacter 0)))
          (Default|AddResource _asbp_char_2 (.RubbishAmount (Utilities|Struct|Breakstruct_PickupItem (Variables|/Game/Blueprints/BP_BaseObject.BP_BaseObject_C|GetItemInfo _output_get_2))))
          (Actor|DestroyActor (Variables|Default|GetBP_BaseObjRef))
          (Development|PrintString "B"))
        (:NewEnumerator2
          (Actor|DestroyActor (Variables|Default|GetBP_BaseObjRef))
          (Development|PrintString "C")
          (bind _asbp_char_3 (Utilities|Casting|CastToBP_Char _returnvalue))
          (Default|AddMotorPart _asbp_char_3))))))

(event OnComponentEndOverlap(Overlap)
  (params (OverlappedComponent :type Primitive%20Component%20Object%20Reference) (OtherActor :type Actor%20Object%20Reference) (OtherComp :type Primitive%20Component%20Object%20Reference) (OtherBodyIndex :type Integer))
  (bind _returnvalue (Game|GetPlayerController 0))
  ;[1 1 1] Player-purifier interaction. Whenever the player is carrying an item. Delete the possessed item if it matches as purifier component. Otherwise ignore everything. Display the caption as soon player overlaps
  (Widget|SetVisibility (Variables|Default|GetWBP_PurifierDisplay) "Hidden")
  (Widget|SetVisibility (Variables|Default|GetWBP_PurifierUIRef) "Hidden")
  (Variables|/Script/Engine.PlayerController|SetbShowMouseCursor _returnvalue false)
  (Variables|/Script/Engine.PlayerController|SetbEnableClickEvents _returnvalue false)
  (Variables|/Script/Engine.PlayerController|SetbEnableMouseOverEvents _returnvalue false))

(event Custom|HandleShowCursor
  (bind _returnvalue (Game|GetPlayerController 0))
  (bind _returnvalue_2 (Game|GetPlayerController 0))
  ;[1 1 1] Handle Cursor
  (if (Utilities|Enum|Equal(Enum) (Widget|GetVisibility (Variables|Default|GetWBP_PurifierUIRef)) "Visible")
    (Variables|/Script/Engine.PlayerController|SetbShowMouseCursor _returnvalue_2 true)
    (Input|SetInputModeGameandUI _returnvalue (Variables|Default|GetWBP_PurifierUIRef) "DoNotLock" true)
    (else
      (Variables|/Script/Engine.PlayerController|SetbShowMouseCursor _returnvalue_2 false)
      (Input|SetInputModeGameOnly _returnvalue))))

(event Custom|CustomEvent_0)

(event EventInteractwithObject
  (bind _wbp_purifieruiref (Variables|Default|GetWBP_PurifierUIRef))
  ;[1 1 1] Toggle purifier
  (Widget|SetVisibility (Variables|Default|GetWBP_PurifierDisplay) "Hidden")
  (if (Utilities|Enum|Equal(Enum) (Widget|GetVisibility (Variables|Default|GetWBP_PurifierUIRef)) "Hidden")
    (Widget|SetVisibility _wbp_purifieruiref "Visible")
    (Variables|Default|SetisHUDOpen true)
    (else
      (Widget|SetVisibility _wbp_purifieruiref "Hidden")
      (Variables|Default|SetisHUDOpen false)))
  (CallFunction|HandleShowCursor)
  (Development|PrintString (Utilities|String|ToString(Boolean) (Variables|Default|GetisHUDOpen))))

(event EventBeginPlay
  ;[1 1 1] Create widgets as soon the game begins
  (bind _returnvalue (UserInterface|CreateWidget "/Game/Blueprints/Devices/Purifier/PurifierUI/WBP_PurifierHUD.WBP_PurifierHUD_C"))
  (bind _output_get (Variables|Default|SetWBP_PurifierUIRef _returnvalue))
  (UserInterface|Viewport|AddtoViewport _returnvalue 0)
  (Widget|SetVisibility _output_get "Hidden")
  (bind _returnvalue_2 (UserInterface|CreateWidget "/Game/Blueprints/Devices/Purifier/PurifierUI/WBP_PurifierDisplay.WBP_PurifierDisplay_C"))
  (bind _output_get_2 (Variables|Default|SetWBP_PurifierDisplay _returnvalue_2))
  (UserInterface|Viewport|AddtoViewport _output_get_2 0)
  (Widget|SetVisibility _returnvalue_2 "Hidden"))

(fn ConstructionScript)

(fn AddResources
  (params (ItemInfo :type Struct%20Pickup%20Item%20Structure))
  (Variables|Default|SetResourceCount (+ (Variables|Default|GetResourceCount) (Utilities|Struct|Breakstruct_PickupItem ItemInfo)))
  (return))