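; BP_Recycler is a recycling device with separate overlap inputs for metal, plastic, glass and paper rubbish.
; Each overlap runs CheckRubbish, which destroys rubbish items and adds matches to RubbishHeld, though plastic and glass amounts land in each other's fields.
; Mismatches are respawned as BP_BaseObject and launched from Output, setting IsSick, which is never cleared here and prints "BLECH!!!!" every tick.
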(event OnComponentBeginOverlap(Metal)
  (params (OverlappedComponent :type Primitive%20Component%20Object%20Reference) (OtherActor :type Actor%20Object%20Reference) (OtherComp :type Primitive%20Component%20Object%20Reference) (OtherBodyIndex :type Integer) (bFromSweep :type Boolean) (SweepResult :type Hit%20Result%20Structure%20%28by%20ref%29))
  (Variables|Default|SetRubbishType "NewEnumerator0")
  (Variables|Default|SetOtherActor OtherActor)
  (bind (_success _item) (CallFunction|CheckRubbish (Variables|Default|GetRubbishType) (Variables|Default|GetOtherActor)))
  (if _success
    (switch Utilities|FlowControl|Switch|SwitchonEnum_RubbishType (.RubbishType (Utilities|Struct|Breakstruct_PickupItem _item))
      (:NewEnumerator0
        (Variables|Default|SetRubbish%20Held (Utilities|Struct|Makestruct_RubbishAmt (+ (.metal (Variables|Default|GetRubbish%20Held)) (.RubbishAmount (Utilities|Struct|Breakstruct_PickupItem _item))) (.glass (Variables|Default|GetRubbish%20Held)) (.plastic (Variables|Default|GetRubbish%20Held)) (.paper (Variables|Default|GetRubbish%20Held)))))
      (:NewEnumerator1
        (Variables|Default|SetRubbish%20Held (Utilities|Struct|Makestruct_RubbishAmt (.metal (Variables|Default|GetRubbish%20Held)) (+ (.glass (Variables|Default|GetRubbish%20Held)) (.RubbishAmount (Utilities|Struct|Breakstruct_PickupItem _item))) (.plastic (Variables|Default|GetRubbish%20Held)) (.paper (Variables|Default|GetRubbish%20Held)))))
      (:NewEnumerator2
        (Variables|Default|SetRubbish%20Held (Utilities|Struct|Makestruct_RubbishAmt (.metal (Variables|Default|GetRubbish%20Held)) (.glass (Variables|Default|GetRubbish%20Held)) (+ (.plastic (Variables|Default|GetRubbish%20Held)) (.RubbishAmount (Utilities|Struct|Breakstruct_PickupItem _item))) (.paper (Variables|Default|GetRubbish%20Held)))))
      (:NewEnumerator3
        (Variables|Default|SetRubbish%20Held (Utilities|Struct|Makestruct_RubbishAmt (.metal (Variables|Default|GetRubbish%20Held)) (.glass (Variables|Default|GetRubbish%20Held)) (.plastic (Variables|Default|GetRubbish%20Held)) (+ (.paper (Variables|Default|GetRubbish%20Held)) (.RubbishAmount (Utilities|Struct|Breakstruct_PickupItem _item)))))))))

(event OnComponentBeginOverlap(Plastic)
  (params (OverlappedComponent :type Primitive%20Component%20Object%20Reference) (OtherActor :type Actor%20Object%20Reference) (OtherComp :type Primitive%20Component%20Object%20Reference) (OtherBodyIndex :type Integer) (bFromSweep :type Boolean) (SweepResult :type Hit%20Result%20Structure%20%28by%20ref%29))
  (Variables|Default|SetRubbishType "NewEnumerator1")
  (Variables|Default|SetOtherActor OtherActor)
  (bind (_success _item) (CallFunction|CheckRubbish (Variables|Default|GetRubbishType) (Variables|Default|GetOtherActor)))
  (if _success
    (switch Utilities|FlowControl|Switch|SwitchonEnum_RubbishType (.RubbishType (Utilities|Struct|Breakstruct_PickupItem _item))
      (:NewEnumerator0
        (Variables|Default|SetRubbish%20Held (Utilities|Struct|Makestruct_RubbishAmt (+ (.metal (Variables|Default|GetRubbish%20Held)) (.RubbishAmount (Utilities|Struct|Breakstruct_PickupItem _item))) (.glass (Variables|Default|GetRubbish%20Held)) (.plastic (Variables|Default|GetRubbish%20Held)) (.paper (Variables|Default|GetRubbish%20Held)))))
      (:NewEnumerator1
        (Variables|Default|SetRubbish%20Held (Utilities|Struct|Makestruct_RubbishAmt (.metal (Variables|Default|GetRubbish%20Held)) (+ (.glass (Variables|Default|GetRubbish%20Held)) (.RubbishAmount (Utilities|Struct|Breakstruct_PickupItem _item))) (.plastic (Variables|Default|GetRubbish%20Held)) (.paper (Variables|Default|GetRubbish%20Held)))))
      (:NewEnumerator2
        (Variables|Default|SetRubbish%20Held (Utilities|Struct|Makestruct_RubbishAmt (.metal (Variables|Default|GetRubbish%20Held)) (.glass (Variables|Default|GetRubbish%20Held)) (+ (.plastic (Variables|Default|GetRubbish%20Held)) (.RubbishAmount (Utilities|Struct|Breakstruct_PickupItem _item))) (.paper (Variables|Default|GetRubbish%20Held)))))
      (:NewEnumerator3
        (Variables|Default|SetRubbish%20Held (Utilities|Struct|Makestruct_RubbishAmt (.metal (Variables|Default|GetRubbish%20Held)) (.glass (Variables|Default|GetRubbish%20Held)) (.plastic (Variables|Default|GetRubbish%20Held)) (+ (.paper (Variables|Default|GetRubbish%20Held)) (.RubbishAmount (Utilities|Struct|Breakstruct_PickupItem _item)))))))))

(event OnComponentBeginOverlap(Glass)
  (params (OverlappedComponent :type Primitive%20Component%20Object%20Reference) (OtherActor :type Actor%20Object%20Reference) (OtherComp :type Primitive%20Component%20Object%20Reference) (OtherBodyIndex :type Integer) (bFromSweep :type Boolean) (SweepResult :type Hit%20Result%20Structure%20%28by%20ref%29))
  (Variables|Default|SetRubbishType "NewEnumerator2")
  (Variables|Default|SetOtherActor OtherActor)
  (bind (_success _item) (CallFunction|CheckRubbish (Variables|Default|GetRubbishType) (Variables|Default|GetOtherActor)))
  (if _success
    (switch Utilities|FlowControl|Switch|SwitchonEnum_RubbishType (.RubbishType (Utilities|Struct|Breakstruct_PickupItem _item))
      (:NewEnumerator0
        (Variables|Default|SetRubbish%20Held (Utilities|Struct|Makestruct_RubbishAmt (+ (.metal (Variables|Default|GetRubbish%20Held)) (.RubbishAmount (Utilities|Struct|Breakstruct_PickupItem _item))) (.glass (Variables|Default|GetRubbish%20Held)) (.plastic (Variables|Default|GetRubbish%20Held)) (.paper (Variables|Default|GetRubbish%20Held)))))
      (:NewEnumerator1
        (Variables|Default|SetRubbish%20Held (Utilities|Struct|Makestruct_RubbishAmt (.metal (Variables|Default|GetRubbish%20Held)) (+ (.glass (Variables|Default|GetRubbish%20Held)) (.RubbishAmount (Utilities|Struct|Breakstruct_PickupItem _item))) (.plastic (Variables|Default|GetRubbish%20Held)) (.paper (Variables|Default|GetRubbish%20Held)))))
      (:NewEnumerator2
        (Variables|Default|SetRubbish%20Held (Utilities|Struct|Makestruct_RubbishAmt (.metal (Variables|Default|GetRubbish%20Held)) (.glass (Variables|Default|GetRubbish%20Held)) (+ (.plastic (Variables|Default|GetRubbish%20Held)) (.RubbishAmount (Utilities|Struct|Breakstruct_PickupItem _item))) (.paper (Variables|Default|GetRubbish%20Held)))))
      (:NewEnumerator3
        (Variables|Default|SetRubbish%20Held (Utilities|Struct|Makestruct_RubbishAmt (.metal (Variables|Default|GetRubbish%20Held)) (.glass (Variables|Default|GetRubbish%20Held)) (.plastic (Variables|Default|GetRubbish%20Held)) (+ (.paper (Variables|Default|GetRubbish%20Held)) (.RubbishAmount (Utilities|Struct|Breakstruct_PickupItem _item)))))))))

(event OnComponentBeginOverlap(Paper)
  (params (OverlappedComponent :type Primitive%20Component%20Object%20Reference) (OtherActor :type Actor%20Object%20Reference) (OtherComp :type Primitive%20Component%20Object%20Reference) (OtherBodyIndex :type Integer) (bFromSweep :type Boolean) (SweepResult :type Hit%20Result%20Structure%20%28by%20ref%29))
  (Variables|Default|SetRubbishType "NewEnumerator3")
  (Variables|Default|SetOtherActor OtherActor)
  (bind (_success _item) (CallFunction|CheckRubbish (Variables|Default|GetRubbishType) (Variables|Default|GetOtherActor)))
  (if _success
    (switch Utilities|FlowControl|Switch|SwitchonEnum_RubbishType (.RubbishType (Utilities|Struct|Breakstruct_PickupItem _item))
      (:NewEnumerator0
        (Variables|Default|SetRubbish%20Held (Utilities|Struct|Makestruct_RubbishAmt (+ (.metal (Variables|Default|GetRubbish%20Held)) (.RubbishAmount (Utilities|Struct|Breakstruct_PickupItem _item))) (.glass (Variables|Default|GetRubbish%20Held)) (.plastic (Variables|Default|GetRubbish%20Held)) (.paper (Variables|Default|GetRubbish%20Held)))))
      (:NewEnumerator1
        (Variables|Default|SetRubbish%20Held (Utilities|Struct|Makestruct_RubbishAmt (.metal (Variables|Default|GetRubbish%20Held)) (+ (.glass (Variables|Default|GetRubbish%20Held)) (.RubbishAmount (Utilities|Struct|Breakstruct_PickupItem _item))) (.plastic (Variables|Default|GetRubbish%20Held)) (.paper (Variables|Default|GetRubbish%20Held)))))
      (:NewEnumerator2
        (Variables|Default|SetRubbish%20Held (Utilities|Struct|Makestruct_RubbishAmt (.metal (Variables|Default|GetRubbish%20Held)) (.glass (Variables|Default|GetRubbish%20Held)) (+ (.plastic (Variables|Default|GetRubbish%20Held)) (.RubbishAmount (Utilities|Struct|Breakstruct_PickupItem _item))) (.paper (Variables|Default|GetRubbish%20Held)))))
      (:NewEnumerator3
        (Variables|Default|SetRubbish%20Held (Utilities|Struct|Makestruct_RubbishAmt (.metal (Variables|Default|GetRubbish%20Held)) (.glass (Variables|Default|GetRubbish%20Held)) (.plastic (Variables|Default|GetRubbish%20Held)) (+ (.paper (Variables|Default|GetRubbish%20Held)) (.RubbishAmount (Utilities|Struct|Breakstruct_PickupItem _item)))))))))

(event Custom|SpitOut
  (params (ItemType :type Struct%20Pickup%20Item%20Structure) (Force :type Float%20%28single-precision%29))
  (bind _returnvalue (Game|SpawnActorfromClass "/Game/Blueprints/BP_BaseObject.BP_BaseObject_C" (Transformation|GetWorldTransform (Variables|Default|GetOutput)) "AdjustIfPossibleButAlwaysSpawn" 0 0))
  (Default|InitialiseObject _returnvalue ItemType)
  (Physics|AddForce (Variables|/Game/Blueprints/BP_BaseObject.BP_BaseObject_C|GetCube _returnvalue) (* (Math|Vector|GetForwardVector (Variables|Default|GetOutput)) Force) "None" false))

(event EventBeginPlay
  (|CallParentFunction) ; This node is disabled and will not be called.\nDrag off pins to build functionality.
)

(event Collision|EventActorBeginOverlap
  (params (OtherActor :type Actor%20Object%20Reference))
  (|CallParentFunction OtherActor) ; This node is disabled and will not be called.\nDrag off pins to build functionality.
)

(event EventTick
  (params (DeltaSeconds :type Float%20%28single-precision%29))
  (|CallParentFunction DeltaSeconds)
  (if (Variables|Default|GetisSick)
    (Development|PrintString "BLECH!!!!")))

(fn ConstructionScript
  (|CallParentFunction))

(fn CheckRubbish
  (params (DesiredTrash :type Enum_RubbishType%20Enum :default "NewEnumerator0") (Actor :type Actor%20Object%20Reference))
  (bind _asbp_base_object (Utilities|Casting|CastToBP_BaseObject Actor))
  (bind _output_get (LocalVariables|SetItemInfo (Variables|/Game/Blueprints/BP_BaseObject.BP_BaseObject_C|GetItemInfo _asbp_base_object)))
  (switch Utilities|FlowControl|Switch|SwitchonEnum_ObjectType (.ObjectType (Utilities|Struct|Breakstruct_PickupItem _output_get))
    (:NewEnumerator0
      (if (== DesiredTrash (.RubbishType (Utilities|Struct|Breakstruct_PickupItem _output_get)))
        (Variables|Default|SetWasSuccessful true)
        (else
          (Variables|Default|SetisSick true)
          (CallFunction|SpitOut (LocalVariables|GetItemInfo) 6e+03)))
      (Actor|DestroyActor Actor)
      (return (== DesiredTrash (.RubbishType (Utilities|Struct|Breakstruct_PickupItem _output_get))) (LocalVariables|GetItemInfo)))))