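; BP_BaseObject is a base item actor that takes its appearance from an ItemInfo data struct.
; InitialiseObject stores the given item info and, when its mesh is valid, applies it to the Cube static mesh component.
; Both the construction script and BeginPlay call it with the current ItemInfo, so the mesh updates in the editor and at runtime.
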(event Custom|InitialiseObject
  (params (Item%20Type :type Struct%20Pickup%20Item%20Structure))
  (bind _mesh (Utilities|Struct|Breakstruct_PickupItem Item%20Type))
  (Variables|Default|SetItemInfo Item%20Type)
  (if (Utilities|IsValid _mesh)
    (Components|StaticMesh|SetStaticMesh (Variables|Default|GetCube) _mesh)))

(event EventBeginPlay
  (CallFunction|InitialiseObject (Variables|Default|GetItemInfo)))

(fn ConstructionScript
  (CallFunction|InitialiseObject (Variables|Default|GetItemInfo)))