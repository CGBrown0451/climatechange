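; Player character that runs on a draining battery, with camera-relative movement, jumping, interaction, pickup carrying and part/resource counters.
; Tick drains battery by base rate, speed and jumping, turns the mesh toward velocity, and updates cameras and the held object.
; Holding Scan switches from spring-arm third person to clamped first person, blocking movement.
; Interact messages overlapping Int_Interaction actors and uses a FlipFlop to grab or release Int_Pickup objects through a PhysicsHandle.
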(event Custom|DrainBattery
  (params (Delta :type Float%20%28single-precision%29))
  (bind _charactermovement (Variables|Character|GetCharacterMovement))
  (bind _returnvalue (Pawn|Components|CharacterMovement|GetLastUpdateVelocity _charactermovement))
  ;[1 1 1] Battery Drain
  (bind _output_get (Variables|Default|SetBattery%20Left (- (Variables|Default|GetBattery%20Left) (+ (* (* (/ (Math|Vector2D|Vector2DLength (Math|Vector2D|MakeVector2D (.x _returnvalue) (.y _returnvalue))) (Class|MovementComponent|GetMaxSpeed _charactermovement)) (Variables|Default|GetMoveDrain)) Delta) (* Delta (Variables|Default|GetBaseDrain))))))
  (if (Variables|Default|GetbWasJumping)
    (bind _output_get_2 (Variables|Default|SetBattery%20Left (- _output_get (* (Variables|Default|GetJumpDrain) Delta))))
    (if (Variables|Default|GetPhysics%20Handle%20Active)
      (Variables|Default|SetBattery%20Left (- _output_get_2 (* 0.0 0.0))))))

(event Custom|OrientationTick
  (bind _charactermovement (Variables|Character|GetCharacterMovement))
  (bind _tppcamera (Variables|Default|GetTPPCamera))
  (bind _fppcamera (Variables|Default|GetFPPCamera))
  (bind _fppcamera_2 (Variables|Default|GetFPPCamera))
  (bind _springarm (Variables|Default|GetSpringArm))
  (bind _returnvalue (Pawn|Components|CharacterMovement|GetLastUpdateVelocity _charactermovement))
  (bind _relativerotation (Variables|/Script/Engine.SceneComponent|GetRelativeRotation _springarm))
  (bind _relativerotation_2 (Variables|/Script/Engine.SceneComponent|GetRelativeRotation _fppcamera_2))
  (bind _returnvalue_2 (Math|Vector|Normalize (Math|Vector|MakeVector (.x _returnvalue) (.y _returnvalue) 0.0)))
  ;[1 1 1] Orientation
  (if (> (Math|Vector|VectorLength _returnvalue_2) 0.0)
    (Variables|Default|SetisStoppped false)
    (Transformation|SetWorldRotation (Variables|Character|GetMesh) (Math|Rotator|MakeRotator 0.0 0.0 (.yaw (Math|Conversions|RotationFromXVector _returnvalue_2))) false false)
    (else
      (Variables|Default|SetisStoppped true)))
  (if (Variables|Default|GetisFPP)
    (Components|Activation|Deactivate _tppcamera)
    (Components|Activation|Activate _fppcamera true)
    (Transformation|SetRelativeRotation _fppcamera_2 (Math|Rotator|MakeRotator 0.0 (Math|Float|Clamp(Float) (.pitch _relativerotation_2) -45.0 45.0) (Math|Float|Clamp(Float) (.yaw _relativerotation_2) -45.0 45.0)) false false)
    (else
      (Components|Activation|Deactivate _fppcamera)
      (Components|Activation|Activate _tppcamera false)
      (Transformation|SetRelativeRotation _fppcamera "0, 0, 0" false false)
      (Transformation|SetRelativeRotation _springarm (Math|Rotator|MakeRotator (.roll _relativerotation) (Math|Float|ClampAngle (.pitch _relativerotation) (Variables|Default|GetTPPMinAngle) (Variables|Default|GetTPPMaxAngle)) (.yaw _relativerotation)) false false))))

(event Custom|PhysicsHandleLocation
  (bind _grabpoint (Variables|Default|GetGrabPoint))
  (bind _returnvalue (Transformation|GetWorldTransform _grabpoint))
  ;[1 1 1] PhysicsHandleTick
  (if (Variables|Default|GetPhysics%20Handle%20Active)
    (Class|PhysicsHandleComponent|SetTargetLocationandRotation (Variables|Default|GetPhysicsHandle) (.location _returnvalue) (.rotation _returnvalue))))

(event Custom|PressInteraction
  (params (Target :type Object%20Object%20Reference))
  ;[1 1 1] PressInteract
  (Development|PrintString "Interacting..." true true "(R=0.112405,G=1.000000,B=0.000000,A=1.000000)" 5.0)
  (Class|IntInteraction|InteractwithObject(Message) Target))

(event EventTick
  (params (DeltaSeconds :type Float%20%28single-precision%29))
  ;[1 1 1] Tick Events
  (CallFunction|DrainBattery DeltaSeconds)
  (CallFunction|OrientationTick)
  (CallFunction|PhysicsHandleLocation))

(event EventBeginPlay
  ;[1 1 1] Beginplay
  (Variables|Default|SetBattery%20Left (Variables|Default|GetBattery%20Life)))

(event Input|ActionEvents|InputActionScan
  (params (Key :type Key%20Structure :default "None"))
  ;[1 1 1] Scan Input
  (:Pressed
    (Variables|Default|SetisFPP true))
  (:Released
    (Variables|Default|SetisFPP false)))

(event Input|ActionEvents|InputActionJump
  (params (Key :type Key%20Structure :default "None"))
  ;[1 1 1] Orientation
  (:Pressed
    (Character|Jump))
  (:Released
    (Character|StopJumping)))

(event Input|ActionEvents|InputActionInteract
  (params (Key :type Key%20Structure :default "None"))
  (bind _interactionzone (Variables|Default|GetInteractionZone))
  (bind _grabpoint (Variables|Default|GetGrabPoint))
  (bind _returnvalue (Transformation|GetWorldTransform _grabpoint))
  ;[1 1 1] GrabbingAndDropping
  (:Pressed
    (bind (_array_element _array_index) (Utilities|Array|ForEachLoopwithBreak (Collision|GetOverlappingActors _interactionzone 0 :!class /Script/Engine.PrimitiveComponent) :!label _label)
      (:LoopBody
        (if (Utilities|DoesObjectImplementInterface _array_element "/Game/Blueprints/Int_Interaction.Int_Interaction_C")
          (CallFunction|PressInteraction _array_element))
        (if (Utilities|DoesObjectImplementInterface _array_element "/Game/Blueprints/Int_pickup.Int_Pickup_C")
          (Utilities|FlowControl|FlipFlop
            (:A
              (if (Utilities|IsValid (Utilities|Array|Get(acopy) (Class|PrimitiveComponent|GetOverlappingComponents _interactionzone) _array_index))
                (Variables|Default|SetPhysics%20Handle%20Active true)
                (Transformation|SetWorldLocationAndRotation (Utilities|Array|Get(acopy) (Class|PrimitiveComponent|GetOverlappingComponents _interactionzone) _array_index) (.location _returnvalue) (.rotation _returnvalue) false false)
                (Physics|Components|PhysicsHandle|GrabComponentatLocationwithRotation (Variables|Default|GetPhysicsHandle) (Utilities|Array|Get(acopy) (Class|PrimitiveComponent|GetOverlappingComponents _interactionzone) _array_index) "None" (.location _returnvalue) (.rotation _returnvalue))
                (if (Utilities|IsValid (Utilities|Array|Get(acopy) (Class|PrimitiveComponent|GetOverlappingComponents _interactionzone) _array_index))
                  (Collision|SetCollisionResponsetoChannel (Utilities|Array|Get(acopy) (Class|PrimitiveComponent|GetOverlappingComponents _interactionzone) _array_index) "ECC_Camera" "ECR_Ignore")
                  (goto _label Break))
                (else
                  (Variables|Default|SetPhysics%20Handle%20Active false :!label _label_2)
                  (Physics|Components|PhysicsHandle|ReleaseComponent (Variables|Default|GetPhysicsHandle)))))
            (:B
              (goto _label_2))))))))

(event Input|AxisEvents|InputAxisLook_Pitch
  (params (AxisValue :type Float%20%28single-precision%29))
  (bind _sensitivity_y (Variables|Default|GetSensitivity_Y))
  (bind _returnvalue (* AxisValue _sensitivity_y))
  ;[1 1 1] Pitch Look
  (if (Variables|Default|GetisFPP)
    (Transformation|AddRelativeRotation (Variables|Default|GetFPPCamera) (Math|Rotator|MakeRotator 0.0 _returnvalue 0.0) false false)
    (else
      (Transformation|AddRelativeRotation (Variables|Default|GetSpringArm) (Math|Rotator|MakeRotator 0.0 _returnvalue 0.0) false false))))

(event Input|AxisEvents|InputAxisLook_Yaw
  (params (AxisValue :type Float%20%28single-precision%29))
  (bind _sensitivity_x (Variables|Default|GetSensitivity_X))
  (bind _returnvalue (* AxisValue _sensitivity_x))
  ;[1 1 1] Yaw Look
  (if (Variables|Default|GetisFPP)
    (Transformation|AddRelativeRotation (Variables|Default|GetFPPCamera) (Math|Rotator|MakeRotator 0.0 0.0 _returnvalue) false false)
    (else
      (Transformation|AddRelativeRotation (Variables|Default|GetSpringArm) (Math|Rotator|MakeRotator 0.0 0.0 _returnvalue) false false))))

(event Input|AxisEvents|InputAxisMove_Forward
  (params (AxisValue :type Float%20%28single-precision%29))
  (bind _springarm (Variables|Default|GetSpringArm))
  (bind _returnvalue (Math|Vector|GetForwardVector _springarm))
  (bind _returnvalue_2 (Math|Vector2D|Normalize2D (Math|Vector2D|MakeVector2D (.x _returnvalue) (.y _returnvalue))))
  ;[1 1 1] Movement
  (if (not (Variables|Default|GetisPurifierHUD_enabled))
    (if (not (Variables|Default|GetisFPP))
      (Pawn|Input|AddMovementInput (Math|Vector|MakeVector (.x _returnvalue_2) (.y _returnvalue_2) 0.0) AxisValue false))))

(event Input|AxisEvents|InputAxisMove_Right
  (params (AxisValue :type Float%20%28single-precision%29))
  (bind _springarm (Variables|Default|GetSpringArm))
  (bind _returnvalue (Math|Vector|GetRightVector _springarm))
  (bind _returnvalue_2 (Math|Vector2D|Normalize2D (Math|Vector2D|MakeVector2D (.x _returnvalue) (.y _returnvalue))))
  ;[1 1 1] Movement
  (if (not (Variables|Default|GetisPurifierHUD_enabled))
    (if (not (Variables|Default|GetisFPP))
      (Pawn|Input|AddMovementInput (Math|Vector|MakeVector (.x _returnvalue_2) (.y _returnvalue_2) 0.0) AxisValue false))))

(fn ConstructionScript)

(fn AddHydraulicPart
  (bind _output_get (Variables|Default|SetAddHydraulic (+ (Variables|Default|GetAddHydraulic) 1)))
  (Development|PrintString (Utilities|String|ToString(Integer) _output_get)))

(fn AddMotorPart
  (bind _output_get (Variables|Default|SetAddMotor (+ (Variables|Default|GetAddMotor) 1)))
  (Development|PrintString (Utilities|String|ToString(Integer) _output_get)))

(fn AddResource
  (params (ItemInfo :type Integer))
  (Variables|Default|SetResourceCount (+ (Variables|Default|GetResourceCount) ItemInfo))
  (Development|PrintString (Utilities|String|ToString(Integer) 0)))